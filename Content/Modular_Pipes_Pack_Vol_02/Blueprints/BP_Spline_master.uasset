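; Master spline Blueprint from a modular pipes pack that repeats a chosen mesh along an editable spline.
; The Construction Script adds one spline mesh component per segment and bends it using the local locations and tangents of that segment's two points.
; Exposed variables set the mesh, forward axis, uniform cross-section width and ten material slot overrides.
; The event graph is empty, so nothing is scripted at runtime.
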(fn `UserConstructionScript`
  (bind _spline (`self.Spline`))
  (bind _mesh_width (`self.Mesh Width`))
  (for _index (range (`SplineComponent.GetNumberOfSplineSegments` (`self.Spline`)))
    (bind _returnvalue (`AddComponent|NODE_AddSplineMeshComponent-0`))
    (`StaticMeshComponent.SetStaticMesh` _returnvalue (`self.Mesh`))
    ;[0.3604 0.6768 1] If you have any custom merged meshes that exceed a total of 10 unique material slots then you can add more to the end here >
    (`PrimitiveComponent.SetMaterial` _returnvalue 0 (`self.Material_slot_01`))
    (`PrimitiveComponent.SetMaterial` _returnvalue 1 (`self.Material_slot_02`))
    (`PrimitiveComponent.SetMaterial` _returnvalue 2 (`self.Material_slot_03`))
    (`PrimitiveComponent.SetMaterial` _returnvalue 3 (`self.Material_slot_04`))
    (`PrimitiveComponent.SetMaterial` _returnvalue 4 (`self.Material_slot_05`))
    (`PrimitiveComponent.SetMaterial` _returnvalue 5 (`self.Material_slot_06`))
    (`PrimitiveComponent.SetMaterial` _returnvalue 6 (`self.Material_slot_07`))
    (`PrimitiveComponent.SetMaterial` _returnvalue 7 (`self.Material_slot_08`))
    (`PrimitiveComponent.SetMaterial` _returnvalue 8 (`self.Material_slot_09`))
    (`PrimitiveComponent.SetMaterial` _returnvalue 9 (`self.Material_slot_10`))
    (`SplineMeshComponent.SetForwardAxis` _returnvalue (`self.Forward Axis`) true)
    (bind (_location _tangent) (`SplineComponent.GetLocationAndTangentAtSplinePoint` _spline _index "Local"))
    (bind (_location_2 _tangent_2) (`SplineComponent.GetLocationAndTangentAtSplinePoint` _spline (+ _index 1) "Local"))
    (`SplineMeshComponent.SetStartAndEnd` _returnvalue _location _tangent _location_2 _tangent_2 true)
    (`SplineMeshComponent.SetStartScale` _returnvalue (`KismetMathLibrary.MakeVector2D` _mesh_width _mesh_width) true)
    (`SplineMeshComponent.SetEndScale` _returnvalue (`KismetMathLibrary.MakeVector2D` _mesh_width _mesh_width) true)))